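; DepositPoint_BP is a drop-off point where the player banks held points as stored points.
; When PlayerCharacter_BP overlaps it, held points times the point multiplier are added to the stored total in NutRun_GI, then held points reset to zero.
; It then updates the player's held-points text and move speed and refreshes its own stored-points text, which is also set on BeginPlay.
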(event Custom|Set%20Stored%20Points%20Text
  (Rendering|Components|TextRender|SetText (Variables|Default|GetStored%20Points) (Utilities|Text|ToText(Integer) (Variables|/Game/Main/NutRun_GI.NutRun_GI_C|GetStoredPoints (Variables|Default|GetGame%20Instance)))))

(event Collision|EventActorBeginOverlap
  (params (OtherActor :type Actor%20Object%20Reference))
  (bind _game_instance (Variables|Default|GetGame%20Instance))
  (bind _asplayer_character_bp (Utilities|Casting|CastToPlayerCharacter_BP OtherActor))
  (Variables|/Game/Main/NutRun_GI.NutRun_GI_C|SetStoredPoints _game_instance (+ (Variables|/Game/Main/NutRun_GI.NutRun_GI_C|GetStoredPoints _game_instance) (* (Variables|/Game/Main/NutRun_GI.NutRun_GI_C|GetHeldPoints _game_instance) (Variables|/Game/Main/NutRun_GI.NutRun_GI_C|GetPointMultiplier _game_instance))))
  (Variables|/Game/Main/NutRun_GI.NutRun_GI_C|SetHeldPoints _game_instance 0)
  (Default|SetHeldPointsText _asplayer_character_bp)
  (Default|ChangeMoveSpeed _asplayer_character_bp)
  (CallFunction|SetStoredPointsText))

(event EventTick
  (params (DeltaSeconds :type Float%20%28single-precision%29)))

(event EventBeginPlay
  (bind _asnut_run_gi (Utilities|Casting|CastToNutRun_GI (Game|GetGameInstance)))
  (Variables|Default|SetGame%20Instance _asnut_run_gi)
  (CallFunction|SetStoredPointsText))

(fn ConstructionScript)