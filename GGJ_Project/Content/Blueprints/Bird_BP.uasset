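; Bird predator actor that hovers above the player and kills them when they stay unhidden too long.
; Each Tick, or on BirdHunt, an attack timer drains while the player is exposed, refills up to TimeToAttack while hidden, and triggers KillPlayer below zero.
; The bird follows at a height offset, spins around yaw, and grows as the timer drops.
; The timer value is printed every update.
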(event Custom|Bird%20Hunt
  (Utilities|FlowControl|Sequence
    (:then_0
      (if (Variables|/Game/Main/PlayerCharacter_BP.PlayerCharacter_BP_C|GetHidden (Variables|Default|GetPlayer))
        (if (>= (Variables|Default|GetAttackTimer) (Variables|Default|GetTimeToAttack))
          (Variables|Default|SetAttackTimer (Variables|Default|GetTimeToAttack))
          (else
            (Variables|Default|SetAttackTimer (+ (Variables|Default|GetAttackTimer) (Utilities|Time|GetWorldDeltaSeconds)))))
        (elif (< (Variables|Default|GetAttackTimer) 0.0)
          (Default|KillPlayer (Variables|Default|GetPlayer))
          (else
            (Variables|Default|SetAttackTimer (- (Variables|Default|GetAttackTimer) (Utilities|Time|GetWorldDeltaSeconds))))))
      (Development|PrintString (Utilities|String|ToString(Float) (Variables|Default|GetAttackTimer))))
    (:then_1
      (CallFunction|SetBirdScale)
      (CallFunction|SetBirdRotation)
      (CallFunction|FollowPlayer))))

(event Custom|SetBirdScale
  (Transformation|SetWorldScale3D (Variables|Default|GetBirdMesh) (Math|Conversions|ToVector(Float) (* (- (+ (Variables|Default|GetTimeToAttack) 1.0) (Variables|Default|GetAttackTimer)) 0.25))))

(event Custom|Follow%20Player
  (bind _player (Variables|Default|GetPlayer))
  (bind _returnvalue (Transformation|GetActorLocation _player))
  (Transformation|SetActorLocation (Math|Vector|MakeVector (.x _returnvalue) (.y _returnvalue) (+ (.z _returnvalue) (Variables|Default|GetZOffset))) false false))

(event Custom|Set%20Bird%20Rotation
  (bind _returnvalue (Transformation|GetActorRotation))
  (Transformation|SetActorRotation (Math|Rotator|MakeRotator (.roll _returnvalue) (.pitch _returnvalue) (+ (.yaw _returnvalue) (* (Utilities|Time|GetWorldDeltaSeconds) (Variables|Default|GetRotationSpeed))))))

(event EventBeginPlay
  (bind _asplayer_character_bp (Utilities|Casting|CastToPlayerCharacter_BP (Game|GetPlayerCharacter 0)))
  (Variables|Default|SetPlayer _asplayer_character_bp))

(event Collision|EventActorBeginOverlap
  (params (OtherActor :type Actor%20Object%20Reference)))

(event EventTick
  (params (DeltaSeconds :type Float%20%28single-precision%29))
  (Utilities|FlowControl|Sequence
    (:then_0
      (if (Variables|/Game/Main/PlayerCharacter_BP.PlayerCharacter_BP_C|GetHidden (Variables|Default|GetPlayer))
        (if (>= (Variables|Default|GetAttackTimer) (Variables|Default|GetTimeToAttack))
          (Variables|Default|SetAttackTimer (Variables|Default|GetTimeToAttack))
          (else
            (Variables|Default|SetAttackTimer (+ (Variables|Default|GetAttackTimer) (Utilities|Time|GetWorldDeltaSeconds)))))
        (elif (< (Variables|Default|GetAttackTimer) 0.0)
          (Default|KillPlayer (Variables|Default|GetPlayer))
          (else
            (Variables|Default|SetAttackTimer (- (Variables|Default|GetAttackTimer) (Utilities|Time|GetWorldDeltaSeconds))))))
      (Development|PrintString (Utilities|String|ToString(Float) (Variables|Default|GetAttackTimer))))
    (:then_1
      (CallFunction|SetBirdScale)
      (CallFunction|SetBirdRotation)
      (CallFunction|FollowPlayer))))

(fn ConstructionScript)